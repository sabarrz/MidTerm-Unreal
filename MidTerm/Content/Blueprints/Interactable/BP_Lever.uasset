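; BP_Lever is an interactable lever Blueprint with a doorLever event that switches it to an up-position mesh and prints a win message.
; A FlipFlop gates the event with only its A output wired, which also clears IsOn and casts the game mode to BP_ThirdPersonGameMode without using the result.
; A down-position branch with a "Door not open yet" message is disconnected and never runs.
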(event `doorLever`
  (`/Engine/EditorBlueprintResources/StandardMacros.FlipFlop`
    (:`A`
      (`StaticMeshComponent.SetStaticMesh` (`self.StaticMeshComponent`) "/Game/SM_Lever_UP_1__1_.SM_Lever_UP_1__1_")
      (set `self.IsOn` false)
      (`KismetSystemLibrary.PrintString` "You Won!")
      (cast `/Game/ThirdPerson/Blueprints/BP_ThirdPersonGameMode` (`GameplayStatics.GetGameMode`)))))

(fn `UserConstructionScript`)