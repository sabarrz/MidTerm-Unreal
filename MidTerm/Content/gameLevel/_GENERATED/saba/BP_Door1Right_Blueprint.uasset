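; BP_Door1Right_Blueprint is a door that moves vertically when its linked button signals open or close.
; On BeginPlay it finds a Cylinder1right_Blueprint_Blueprint actor by class and binds Open and Close to that button's events.
; Each event uses MoveComponentTo to shift the static mesh 500 units up or down from its current position.
; The target is computed from world location but passed as a relative location.
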(event `self.ReceiveBeginPlay`
  (bind _returnvalue (`GameplayStatics.GetActorOfClass` "/Game/gameLevel/_GENERATED/saba/Cylinder1right_Blueprint_Blueprint.Cylinder1right_Blueprint_Blueprint_C"))
  (bind _output_get (set `self.Button` _returnvalue))
  (add `/Game/gameLevel/_GENERATED/saba/Cylinder1left_Blueprint.Open` _output_get (delegate `Open`))
  (add `/Game/gameLevel/_GENERATED/saba/Cylinder1left_Blueprint.Close` _output_get (delegate `Close`)))

(event `Open`
  (bind _staticmeshcomponent (`self.StaticMeshComponent`))
  (`KismetSystemLibrary.MoveComponentTo` _staticmeshcomponent (+ (`SceneComponent.K2_GetComponentLocation` _staticmeshcomponent) (0.0 0.0 500.0))))

(event `Close`
  (bind _staticmeshcomponent (`self.StaticMeshComponent`))
  (`KismetSystemLibrary.MoveComponentTo` _staticmeshcomponent (+ (`SceneComponent.K2_GetComponentLocation` _staticmeshcomponent) (0.0 0.0 -500.0))))

(fn `UserConstructionScript`)